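; Player pawn that keeps moving along a world axis after a single key press until its capsule hits something.
; Four input actions set a Direction state and signed Scale, and capsule hits reset Direction to Null.
; Each Tick, MoveInDirection applies world X or Y input and sets rotation from the actor's own scaled forward or right vector.
; When Null, it reapplies the stored rotation and prints a debug message.
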(event OnComponentHit(CapsuleComponent)
  (params (HitComponent :type Primitive%20Component%20Object%20Reference) (OtherActor :type Actor%20Object%20Reference) (OtherComp :type Primitive%20Component%20Object%20Reference) (NormalImpulse :type Vector :default "0, 0, 0") (Hit :type Hit%20Result%20Structure%20%28by%20ref%29))
  (Variables|Default|SetDirection "NewEnumerator2"))

(event EventTick
  (params (DeltaSeconds :type Float%20%28single-precision%29))
  (CallFunction|MoveinDirection (Variables|Default|GetDirection) (Variables|Default|GetScale)))

(event EventBeginPlay
  (Variables|Default|SetDirection "NewEnumerator2"))

(event Input|ActionEvents|InputActionSR
  (params (Key :type Key%20Structure :default "None"))
  (:Pressed
    (Variables|Default|SetDirection "NewEnumerator1")
    (Variables|Default|SetScale 1.0)))

(event Input|ActionEvents|InputActionSL
  (params (Key :type Key%20Structure :default "None"))
  (:Pressed
    (Variables|Default|SetDirection "NewEnumerator1")
    (Variables|Default|SetScale -1.0)))

(event Input|ActionEvents|InputActionFW
  (params (Key :type Key%20Structure :default "None"))
  (:Pressed
    (Variables|Default|SetDirection "NewEnumerator0")
    (Variables|Default|SetScale 1.0)))

(event Input|ActionEvents|InputActionBW
  (params (Key :type Key%20Structure :default "None"))
  (:Pressed
    (Variables|Default|SetDirection "NewEnumerator0")
    (Variables|Default|SetScale -1.0)))

(fn ConstructionScript)

(fn MoveinDirection
  (params (Direction :type EDirection%20Enum :default "NewEnumerator2") (scale :type Float%20%28single-precision%29))
  (switch Utilities|FlowControl|Switch|SwitchonEDirection Direction
    (:NewEnumerator2
      (Development|PrintString "Player is still" true true "(R=0.000000,G=0.660000,B=1.000000,A=1.000000)" 0.0)
      (Transformation|SetActorRotation (Variables|Default|GetCurrent%20Rotation)))
    (:NewEnumerator0
      (Pawn|Input|AddMovementInput (Math|Vector|MakeVector 1.0 0.0 0.0) scale false)
      (bind _output_get (Variables|Default|SetCurrent%20Rotation (Math|Conversions|RotationFromXVector (* (Math|Vector|Normalize (Transformation|GetActorForwardVector)) (Variables|Default|GetScale)))))
      (Transformation|SetActorRotation _output_get))
    (:NewEnumerator1
      (Pawn|Input|AddMovementInput (Math|Vector|MakeVector 0.0 1.0 0.0) scale false)
      (bind _output_get_2 (Variables|Default|SetCurrent%20Rotation (Math|Conversions|RotationFromXVector (* (Math|Vector|Normalize (Transformation|GetActorRightVector)) (Variables|Default|GetScale)))))
      (Transformation|SetActorRotation _output_get_2))))